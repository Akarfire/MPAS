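; Debug visualizer component for MPAS rigs that spawns collision-free meshes on its owner for each visible rig element.
; Limbs get one length-scaled mesh per segment, tagged with its index and moved each Tick to the limb's current state.
; Other elements get attached cubes for body segments or spheres otherwise.
; Separate functions print position and rotation stack layers, with debug spheres drawn for positions.
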(event `self.ReceiveTick`
  (params (DeltaSeconds :type "Float (single-precision)"))
  (bind _limbvissegments (`self.LimbVisSegments`))
  (bind _keys (`BlueprintMapLibrary.Map_Keys` _limbvissegments))
  (for _array_element _keys
    (bind (_location _rotation) (break `MPAS_LimbSegmentState` (`|GetArrayItem` (`MPAS_Limb.GetCurrentState` (`BlueprintMapLibrary.Map_Find` _limbvissegments _array_element)) (`KismetStringLibrary.Conv_StringToInt` (`KismetStringLibrary.Conv_NameToString` (`|GetArrayItem` (`ActorComponent.ComponentTags` _array_element)))))))
    (`SceneComponent.K2_SetWorldLocationAndRotation` _array_element _location _rotation false false)))

(fn `Debug Position Stack`
  (params (Target :type "MPAS_RigElement Object Reference") (InPositionStackID :type Integer))
  (locals (CurrentLine :type String))
  (bind _output (`|GetArrayItem` (`MPAS_RigElement.VectorStacks` Target) InPositionStackID))
  (`/Engine/EditorBlueprintResources/StandardMacros.IsValid` Target
    (:`Is Valid`
      (for _array_element (`MPAS_RigElement.DEBUG_GetVectorStackExecutionOrder` Target InPositionStackID)
        (set `local.CurrentLine` (`KismetStringLibrary.Concat_StrStr` (`KismetStringLibrary.Conv_IntToString` _array_element) " -  " (`KismetStringLibrary.Conv_NameToString` (`StacksAndLayers.GetLayerName_Vector` _output _array_element)) ":   "))
        (bind _returnvalue (`StacksAndLayers.GetLayerElements_Vector` _output _array_element))
        (bind _keys (`BlueprintMapLibrary.Map_Keys` _returnvalue))
        (for _array_element_2 _keys
          (bind _value (`BlueprintMapLibrary.Map_Find` _returnvalue _array_element_2))
          (set `local.CurrentLine` (`KismetStringLibrary.Concat_StrStr` (`local.CurrentLine`) (`KismetSystemLibrary.GetObjectName` _array_element_2) " - " (`KismetStringLibrary.Conv_VectorToString` _value) "   ,   " (select `int` _ :`0` "" :`1` "") "   ,   "))
          (bind _returnvalue_2 (select `int` (mod _array_element 4) :`0` (struct :`G` 0.384577 :`B` 1.0 :`A` 1.0) :`1` (struct :`R` 0.09448 :`B` 1.0 :`A` 1.0) :`2` (struct :`R` 0.969136 :`B` 1.0 :`A` 1.0) :`3` (struct :`R` 1.0 :`B` 0.034265 :`A` 1.0) :!type "LinearColor Structure"))
          (`KismetSystemLibrary.DrawDebugSphere` _value 100.0 0 _returnvalue_2 0.0 5.0))
        (`KismetSystemLibrary.PrintString` (`KismetStringLibrary.Concat_StrStr` (`local.CurrentLine`) "" (`KismetStringLibrary.Conv_BoolToString` (`StacksAndLayers.GetLayerEnabled_Vector` _output _array_element)) ", " (`KismetStringLibrary.Conv_DoubleToString` (`StacksAndLayers.GetLayerBlendingFactor_Vector` _output _array_element))) true true _returnvalue_2 0.0))
      (`KismetSystemLibrary.DrawDebugSphere` (`StacksAndLayers.CalculateStack_Vector` _output) 150.0 0 (struct :`G` 1.0 :`B` 0.059495 :`A` 1.0) 0.0 5.0))))

(fn `DebugRotationStack`
  (params (Target :type "MPAS_RigElement Object Reference") (InRotationStackID :type Integer))
  (locals (CurrentLine :type String))
  (bind _output (`|GetArrayItem` (`MPAS_RigElement.RotatorStacks` Target) InRotationStackID))
  (`/Engine/EditorBlueprintResources/StandardMacros.IsValid` Target
    (:`Is Valid`
      (for _array_element (`MPAS_RigElement.DEBUG_GetVectorStackExecutionOrder` Target InRotationStackID)
        (set `local.CurrentLine` (`KismetStringLibrary.Concat_StrStr` (`KismetStringLibrary.Conv_NameToString` (`StacksAndLayers.GetLayerName_Rotator` _output _array_element)) ":   "))
        (bind _returnvalue (`StacksAndLayers.GetLayerElements_Rotator` _output _array_element))
        (bind _keys (`BlueprintMapLibrary.Map_Keys` _returnvalue))
        (for _array_element_2 _keys
          (set `local.CurrentLine` (`KismetStringLibrary.Concat_StrStr` (`local.CurrentLine`) (`KismetSystemLibrary.GetObjectName` _array_element_2) " - " (`KismetStringLibrary.Conv_RotatorToString` (`BlueprintMapLibrary.Map_Find` _returnvalue _array_element_2)) "   ,   ")))
        (`KismetSystemLibrary.PrintString` (`local.CurrentLine`) true true (struct :`G` 0.66 :`B` 1.0 :`A` 1.0) 0.0)))))

(fn `GenerateRigVisualization`
  (params (Handler :type "MPAS_Handler Object Reference"))
  (bind _values (`BlueprintMapLibrary.Map_Values` (`MPAS_Handler.GetRigData` (`local.Handler`))))
  (for _array_element _values
    (bind ((`RigElement` _rigelement)) (break `MPAS_RigElementData` _array_element))
    (if (`SceneComponent.IsVisible` _rigelement)
      (bind _asmpas_limb (cast `MPAS_Limb` _rigelement)
        (:`then`
          (for (_array_element_2 _array_index) (`MPAS_Limb.Segments` _asmpas_limb)
            (bind _returnvalue (`|AddComponentByClass` (`self.GetOwner`) "/Script/Engine.StaticMeshComponent" true (`KismetMathLibrary.MakeTransform` (0.0 0.0 0.0) (struct) (`KismetMathLibrary.MakeVector_NetQuantize` (* (`.Length` (break `MPAS_LimbSegmentData` _array_element_2)) 0.01) 0.5 0.5))))
            (`BlueprintMapLibrary.Map_Add` (`self.LimbVisSegments`) _returnvalue _asmpas_limb)
            (`PrimitiveComponent.SetCollisionEnabled` _returnvalue "NoCollision")
            (`StaticMeshComponent.SetStaticMesh` _returnvalue "/MPAS/Mesh/MPAS_PhysicsLimbSegmentMesh_Rectange.MPAS_PhysicsLimbSegmentMesh_Rectange")
            (`KismetArrayLibrary.Array_Add` (`ActorComponent.ComponentTags` _returnvalue) (`KismetStringLibrary.Conv_StringToName` (`KismetStringLibrary.Conv_IntToString` _array_index)))))
        (:`CastFailed`
          (bind _returnvalue_2 (`|AddComponentByClass` :`self` (`self.GetOwner`) :`Class` "/Script/Engine.StaticMeshComponent" :`bManualAttachment` true))
          (`PrimitiveComponent.SetCollisionEnabled` _returnvalue_2 "NoCollision")
          (`SceneComponent.K2_AttachToComponent` _returnvalue_2 _rigelement "None" "SnapToTarget" "SnapToTarget" "SnapToTarget" true)
          (cast `MPAS_BodySegment` _rigelement
            (:`then`
              (`StaticMeshComponent.SetStaticMesh` _returnvalue_2 "/Game/TP/Geometry/Meshes/1M_Cube.1M_Cube")
              (`SceneComponent.SetRelativeScale3D` _returnvalue_2 (1.5 1.5 1.5)))
            (:`CastFailed`
              (`StaticMeshComponent.SetStaticMesh` _returnvalue_2 "/Game/Zaris/Particles/Meshes/Blender_Sphere.Blender_Sphere")
              (`SceneComponent.SetRelativeScale3D` _returnvalue_2 (0.5 0.5 0.5))))))))
  (return))